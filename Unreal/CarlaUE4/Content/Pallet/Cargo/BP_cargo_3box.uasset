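; BP_cargo_3box is a procedural pallet cargo prop that builds a randomized box stack in its construction script.
; It places one large box beside a pair of smaller boxes, with a MultiGate randomly choosing one or two layers for the pair.
; CreateRandomBox adds each mesh with random variant, quarter-turn and transform jitter.
; A rolled hue value is shared by all boxes, except 1.0, which gives each box a random palette hue.
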(event EventBeginPlay)

(event Collision|EventActorBeginOverlap
  (params (OtherActor :type Actor%20Object%20Reference)))

(event EventTick
  (params (DeltaSeconds :type Float%20%28single-precision%29)))

(fn ConstructionScript
  (bind _scale_offset (LocalVariables|GetScale_offset))
  (bind _position_offset (LocalVariables|GetPosition_offset))
  (bind _rotation_offset (LocalVariables|GetRotation_offset))
  (bind _returnvalue (CallFunction|StaticRandom(float)))
  (bind _returnvalue_2 (CallFunction|StaticRandom(element) (Utilities|Array|MakeArray _returnvalue 0.0 1.0)))
  (Utilities|FlowControl|MultiGate true false -1
    (:Out%200
      (Utilities|CreateBoxTopLayer _position_offset _rotation_offset "0.100000,0.100000,0.400000" 14.4 false _returnvalue_2))
    (:Out%201
      (bind _height_z (Utilities|CreateBoxLayer _position_offset _rotation_offset _scale_offset 14.4 _returnvalue_2))
      (Utilities|CreateBoxTopLayer _position_offset _rotation_offset _scale_offset (+ _height_z 14.4) false _returnvalue_2)))
  (Utilities|CreateRandomBox :Position "0,-20.000000,14.400000" :Position_offset _position_offset :Rotation_offset _rotation_offset :Scale "1.000000,1.000000,1.000000" :Scale_offset _scale_offset :Hue_offset _returnvalue_2))