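; Cargo pallet Blueprint that builds a randomized row of one to four bikes in its construction script.
; A random MultiGate picks the layout, with repeated outputs weighting the odds toward more bikes.
; CreateRandomBike adds each static mesh with jittered position and rotation, random scale and a "Base Color" tint, and disables decals.
; Bikes in multi-bike rows also randomly flip 180 degrees in yaw.
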(event EventBeginPlay)

(event Collision|EventActorBeginOverlap
  (params (OtherActor :type Actor%20Object%20Reference)))

(event EventTick
  (params (DeltaSeconds :type Float%20%28single-precision%29)))

(fn ConstructionScript
  (bind _returnvalue (Math|Random|RandomInteger 2))
  (bind _returnvalue_2 (* _returnvalue 1.8e+02))
  (bind _returnvalue_3 (+ _returnvalue_2 9e+01))
  (bind _returnvalue_4 (Math|Vector|MakeVector 0.0 0.0 _returnvalue_3))
  (bind _returnvalue_5 (CallFunction|StaticRandom(color)))
  (bind _returnvalue_6 (CallFunction|StaticRandom(float)))
  (Utilities|FlowControl|MultiGate true false -1
    (:Out%200
      (Utilities|CreateRandomBike :Position "0.000000,0.000000,14.400000" :Position_offset "5.000000,5.000000,0.000000" :Rotation "0,0,90.000000" :Scale (Math|Vector|MakeVector (- 1.0 (* _returnvalue_6 0.2)) (- 1.0 (* _returnvalue_6 0.2)) (- 1.0 (* _returnvalue_6 0.2))) :Color _returnvalue_5))
    (:Out%201
      (Utilities|CreateRandomBike "-20.000000,0.000000,14.400000" "5.000000,5.000000,0.000000" _returnvalue_4 "0.000000,2.000000,5.000000" (Math|Vector|MakeVector (- 1.0 (* _returnvalue_6 0.2)) (- 1.0 (* _returnvalue_6 0.2)) (- 1.0 (* _returnvalue_6 0.2))) _returnvalue_5 :!label _label)
      (Utilities|CreateRandomBike "20.000000,0.000000,14.400000" "5.000000,5.000000,0.000000" _returnvalue_4 "0.000000,2.000000,5.000000" (Math|Vector|MakeVector (- 1.0 (* _returnvalue_6 0.2)) (- 1.0 (* _returnvalue_6 0.2)) (- 1.0 (* _returnvalue_6 0.2))) _returnvalue_5))
    (:Out%202
      (goto _label))
    (:Out%203
      (Utilities|CreateRandomBike "-25.000000,0.000000,14.400000" "5.000000,5.000000,0.000000" _returnvalue_4 "0.000000,2.000000,5.000000" (Math|Vector|MakeVector (- 1.0 (* _returnvalue_6 0.2)) (- 1.0 (* _returnvalue_6 0.2)) (- 1.0 (* _returnvalue_6 0.2))) _returnvalue_5 :!label _label_2)
      (Utilities|CreateRandomBike "0.000000,0.000000,14.400000" "5.000000,5.000000,0.000000" _returnvalue_4 "0.000000,2.000000,5.000000" (Math|Vector|MakeVector (- 1.0 (* _returnvalue_6 0.2)) (- 1.0 (* _returnvalue_6 0.2)) (- 1.0 (* _returnvalue_6 0.2))) _returnvalue_5)
      (Utilities|CreateRandomBike "25.000000,0.000000,14.400000" "5.000000,5.000000,0.000000" _returnvalue_4 "0.000000,2.000000,5.000000" (Math|Vector|MakeVector (- 1.0 (* _returnvalue_6 0.2)) (- 1.0 (* _returnvalue_6 0.2)) (- 1.0 (* _returnvalue_6 0.2))) _returnvalue_5))
    (:Out%204
      (goto _label_2))
    (:Out%205
      (goto _label_2))
    (:Out%206
      (Utilities|CreateRandomBike "-30.000000,0.000000,14.400000" "5.000000,5.000000,0.000000" _returnvalue_4 "0.000000,2.000000,5.000000" (Math|Vector|MakeVector (- 1.0 (* _returnvalue_6 0.2)) (- 1.0 (* _returnvalue_6 0.2)) (- 1.0 (* _returnvalue_6 0.2))) _returnvalue_5 :!label _label_3)
      (Utilities|CreateRandomBike "-10.000000,0.000000,14.400000" "5.000000,5.000000,0.000000" _returnvalue_4 "0.000000,2.000000,5.000000" (Math|Vector|MakeVector (- 1.0 (* _returnvalue_6 0.2)) (- 1.0 (* _returnvalue_6 0.2)) (- 1.0 (* _returnvalue_6 0.2))) _returnvalue_5)
      (Utilities|CreateRandomBike "10.000000,0.000000,14.400000" "5.000000,5.000000,0.000000" _returnvalue_4 "0.000000,2.000000,5.000000" (Math|Vector|MakeVector (- 1.0 (* _returnvalue_6 0.2)) (- 1.0 (* _returnvalue_6 0.2)) (- 1.0 (* _returnvalue_6 0.2))) _returnvalue_5)
      (Utilities|CreateRandomBike "30.000000,0.000000,14.400000" "5.000000,5.000000,0.000000" _returnvalue_4 "0.000000,2.000000,5.000000" (Math|Vector|MakeVector (- 1.0 (* _returnvalue_6 0.2)) (- 1.0 (* _returnvalue_6 0.2)) (- 1.0 (* _returnvalue_6 0.2))) _returnvalue_5))
    (:Out%207
      (goto _label_3))
    (:Out%208
      (goto _label_3))
    (:Out%209
      (goto _label_3))))